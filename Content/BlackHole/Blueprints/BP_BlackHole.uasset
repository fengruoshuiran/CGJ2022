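; Black hole actor that applies its material to a mesh and drives a cube scene capture, likely to supply that material's view of the background.
; Each Tick with SceneCapture set, it moves the capture to the player pawn as a camera stand-in and scans every actor in the level.
; Actors nearer than the black hole and in its facing hemisphere, except SkyboxActor, are hidden from the capture along with itself.
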(event EventBeginPlay)

(event Collision|EventActorBeginOverlap
  (params (OtherActor :type Actor%20Object%20Reference)))

(event EventTick
  (params (DeltaSeconds :type Float%20%28single-precision%29))
  (bind _self self)
  (bind _scc (Variables|Default|GetSCC))
  (bind _skybox_actor (Variables|Default|GetSkybox_Actor))
  (bind _returnvalue (Transformation|GetActorLocation _self))
  (bind _returnvalue_2 (Transformation|GetActorLocation _scc))
  (if (Variables|Default|GetSceneCapture)
    (Transformation|SetActorLocation (Variables|Default|GetSCC) (Transformation|GetActorLocation (Game|Player|GetPlayerPawn 0)) false false)
    (Utilities|Array|Clear (Variables|Default|GetArr_Near_Actors))
    (bind _outactors (Actor|GetAllActorsOfClass "/Script/Engine.Actor"))
    (for _array_element _outactors
      (if (< (Math|Vector|Distance(Vector) (Transformation|GetActorLocation _array_element) _returnvalue_2) (Math|Vector|Distance(Vector) _returnvalue _returnvalue_2))
        (if (> (Math|Vector|DotProduct (Class|KismetMathLibrary|VectorNormalUnsafe (- _returnvalue_2 _returnvalue)) (Class|KismetMathLibrary|VectorNormalUnsafe (- _returnvalue_2 (Transformation|GetActorLocation _array_element)))) 0.0)
          (if (== _skybox_actor 0)
            (Utilities|Array|Add (Variables|Default|GetArr_Near_Actors) _array_element :!label _label)
            (elif (not (== _skybox_actor _array_element))
              (goto _label))))))
    (Utilities|Array|Add (Variables|Default|GetArr_Near_Actors) self)
    (Variables|/Script/Engine.SceneCaptureComponent|SetHiddenActors (Variables|/Script/Engine.SceneCaptureCube|GetCaptureComponentCube (Variables|Default|GetSCC)) (Variables|Default|GetArr_Near_Actors))))

(fn ConstructionScript
  (Rendering|Material|SetMaterial (Variables|Default|GetBlack%20Hole%20Mesh) 0 (Variables|Default|GetBlack%20Hole%20Material)))