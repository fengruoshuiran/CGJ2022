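; Main game mode that sets up each level and handles its win and lose screens.
; On BeginPlay it reads the level name from BP_LevelInfo, spawns and possesses BP_Manny at BP_PlayerStart, and switches view to a spawned follow camera.
; It spawns a delay system bound to the character, then passes both to a detection actor; floor spawning is disconnected.
; Win or lose events show their widget with UI-only input and pause the game.
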(event Custom|Event%20player%20lose
  (bind _returnvalue (Game|GetPlayerController 0))
  (Utilities|IsValid (Variables|Default|GetWB_Lose)
    (:Is%20Valid
      _)
    (:Is%20Not%20Valid
      (bind _returnvalue_2 (UserInterface|CreateWidget "/Game/WB/WB_LOSE.WB_LOSE_C"))
      (Variables|Default|SetWB_Lose _returnvalue_2)))
  (UserInterface|Viewport|AddtoViewport (Variables|Default|GetWB_Lose) 0)
  (Input|SetInputModeUIOnly _returnvalue (Variables|Default|GetWB_Lose) "DoNotLock")
  (Variables|/Script/Engine.PlayerController|SetbShowMouseCursor _returnvalue true)
  (Game|SetGamePaused true))

(event Custom|Event%20player%20win
  (bind _returnvalue (Game|GetPlayerController 0))
  (Utilities|IsValid (Variables|Default|GetWB_WIN)
    (:Is%20Valid
      _)
    (:Is%20Not%20Valid
      (bind _returnvalue_2 (UserInterface|CreateWidget "/Game/WB/WB_WIN.WB_WIN_C" 0 (Variables|Default|Getlevel%20index)))
      (Variables|Default|SetWB_WIN _returnvalue_2)))
  (UserInterface|Viewport|AddtoViewport (Variables|Default|GetWB_WIN) 0)
  (Input|SetInputModeUIOnly _returnvalue (Variables|Default|GetWB_WIN) "DoNotLock")
  (Variables|/Script/Engine.PlayerController|SetbShowMouseCursor _returnvalue true)
  (Game|SetGamePaused true))

(event EventBeginPlay
  ;[0.02783 1 0] Initial
  (CallFunction|Initial))

(fn ConstructionScript)

(fn Initial
  (bind _returnvalue (Game|GetPlayerController 0))
  (bind _returnvalue_2 (Game|GetPlayerController 0))
  (Utilities|FlowControl|Sequence
    (:then_0
      (Input|SetInputModeGameOnly _returnvalue_2)
      (Variables|/Script/Engine.PlayerController|SetbShowMouseCursor _returnvalue_2 false))
    (:then_1
      (bind _outactors (Actor|GetAllActorsOfClass "/Game/BP/BP_LevelInfo.BP_LevelInfo_C"))
      (Variables|Default|Setlevel%20index (Variables|/Game/BP/BP_LevelInfo.BP_LevelInfo_C|Getlevel%20name (Utilities|Array|Get(acopy) _outactors))))
    (:then_2
      (bind _outactors_2 (Actor|GetAllActorsOfClass "/Game/BP/BP_PlayerStart.BP_PlayerStart_C"))
      (Variables|Default|SetSpawnTransform (Math|Transform|MakeTransform (Transformation|GetActorLocation (Utilities|Array|Get(acopy) _outactors_2)))))
    (:then_3
      (bind _returnvalue_3 (Game|SpawnActorfromClass "/Game/BP/BP_Manny.BP_Manny_C" (Variables|Default|GetSpawnTransform) "Undefined" 0 0))
      (bind _output_get (Variables|Default|SetBP_Manny _returnvalue_3))
      (Pawn|Possess _returnvalue _output_get)
      (Variables|/Game/BP/BP_Manny.BP_Manny_C|SetStartLocation _output_get (.Location (Math|Transform|BreakTransform (Variables|Default|GetSpawnTransform)))))
    (:then_4
      (bind _returnvalue_4 (Game|SpawnActorfromClass "/Game/BP/BP_Camera.BP_Camera_C" (Variables|Default|GetSpawnTransform) "Undefined" 0 (Variables|Default|GetBP_Manny) 0))
      (bind _output_get_2 (Variables|Default|SetBP_Camera _returnvalue_4))
      (Game|Player|SetViewTargetwithBlend _returnvalue _output_get_2 0.0 "VTBlend_Linear" 0.0 false)
      (Variables|/Game/BP/BP_Camera.BP_Camera_C|SetbEnableFollow _output_get_2 true))
    (:then_5
      (bind _returnvalue_5 (Game|SpawnActorfromClass "/Game/BP/BP_DelaySystem.BP_DelaySystem_C" (Variables|Default|GetSpawnTransform) "Undefined" 0 (Variables|Default|GetBP_Manny) 0))
      (Variables|Default|SetBP_DelaySystem _returnvalue_5))
    (:then_6
      (bind _returnvalue_6 (Game|SpawnActorfromClass "/Game/BP/BP_Detection.BP_Detection_C" (Variables|Default|GetSpawnTransform) "Undefined" 0 (Variables|Default|Getdetection%20radius) (Variables|Default|GetBP_Manny) (Variables|Default|GetBP_DelaySystem) 3.0 0))
      (Variables|Default|Setbe%20detection%20ref _returnvalue_6))))