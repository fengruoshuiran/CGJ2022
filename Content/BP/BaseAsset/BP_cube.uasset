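; BP_cube is an actor whose Cube component animates vertically when it spawns and again before it is removed.
; On BeginPlay a sped-up timeline drives the cube's relative Z without sweeping.
; The disapperCube event plays a second sped-up timeline that moves the cube along Z with sweep enabled, then destroys the actor when finished.
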(event Custom|disapperCube
  (Components|Timeline|SetPlayRate (Variables|Default|GetTimeline_1) 3.0)
  (bind _newtrack_0 (Timeline|Timeline_1 PlayFromStart)
    (:Update
      (Transformation|SetRelativeLocation (Variables|Default|GetCube) (Math|Vector|MakeVector 0.0 0.0 _newtrack_0) true false))
    (:Finished
      (Actor|DestroyActor))))

(event EventBeginPlay
  (Components|Timeline|SetPlayRate (Variables|Default|GetTimeline_0) 5.0)
  (bind _newtrack_0 (Timeline|Timeline_0 PlayFromStart)
    (:Update
      (Transformation|SetRelativeLocation (Variables|Default|GetCube) (Math|Vector|MakeVector 0.0 0.0 _newtrack_0) false false))))

(fn ConstructionScript)