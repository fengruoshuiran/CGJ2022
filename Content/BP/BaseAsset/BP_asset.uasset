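; Base asset Blueprint that fades a static mesh in and out through a material opacity parameter.
; The construction script creates a dynamic instance of M_Master on the mesh and starts it fully transparent.
; Turnon plays a timeline that drives Opacity on that instance and prints a debug string when finished, while Turnoff reverses it.
; BeginPlay sets a timeline play rate to speed up playback.
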(event Custom|Turn%20off
  (bind _newtrack_0 (Timeline|Timeline_0 Reverse)
    (:Update
      (bind _output_get (Variables|Default|SetOpacity _newtrack_0))
      (Rendering|Material|SetScalarParameterValue (Variables|Default|GetMID_asset) "Opacity" _output_get :!class /Script/Engine.MaterialInstanceDynamic))
    (:Finished
      (Development|PrintString "Hello"))))

(event Custom|Turn%20on
  (bind _newtrack_0 (Timeline|Timeline_0 Play)
    (:Update
      (bind _output_get (Variables|Default|SetOpacity _newtrack_0))
      (Rendering|Material|SetScalarParameterValue (Variables|Default|GetMID_asset) "Opacity" _output_get :!class /Script/Engine.MaterialInstanceDynamic))
    (:Finished
      (Development|PrintString "Hello"))))

(event EventBeginPlay
  (Components|Timeline|SetPlayRate (Variables|Default|GetTimeline_0) 2.0))

(fn ConstructionScript
  (bind _returnvalue (Rendering|Material|CreateDynamicMaterialInstance (Variables|Default|GetStaticMesh) 0 "/Game/BP/BaseAsset/M_Master.M_Master" "MI_Master" :!class /Script/Engine.PrimitiveComponent))
  (bind _output_get (Variables|Default|SetMID_asset _returnvalue))
  (Rendering|Material|SetScalarParameterValue _output_get "Opacity" 0.0 :!class /Script/Engine.MaterialInstanceDynamic))