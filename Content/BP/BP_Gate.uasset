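; BP_Gate is a gate that opens while the player pawn is inside its trigger and closes after a short delay once the player leaves.
; The trigger overlaps set an open flag, and Tick either plays the timeline or counts down Power before reversing it.
; The timeline lerps the door's relative Z from its BeginPlay position to DoorHeight.
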(event OnComponentBeginOverlap(Triger)
  (params (OverlappedComponent :type Primitive%20Component%20Object%20Reference) (OtherActor :type Actor%20Object%20Reference) (OtherComp :type Primitive%20Component%20Object%20Reference) (OtherBodyIndex :type Integer) (bFromSweep :type Boolean) (SweepResult :type Hit%20Result%20Structure%20%28by%20ref%29))
  (if (== OtherActor (Game|Player|GetPlayerPawn 0))
    (Variables|Default|SetPower 2.0)
    (Variables|Default|SetIsOpen? true)))

(event OnComponentEndOverlap(Triger)
  (params (OverlappedComponent :type Primitive%20Component%20Object%20Reference) (OtherActor :type Actor%20Object%20Reference) (OtherComp :type Primitive%20Component%20Object%20Reference) (OtherBodyIndex :type Integer))
  (if (== OtherActor (Game|Player|GetPlayerPawn 0))
    (Variables|Default|SetIsOpen? false)))

(event EventBeginPlay
  (Variables|Default|SetInitial%20location (Variables|/Script/Engine.SceneComponent|GetRelativeLocation (Variables|Default|GetDoor))))

(event EventTick
  (params (DeltaSeconds :type Float%20%28single-precision%29))
  (bind _initial_location (Variables|Default|GetInitial%20location))
  (bind (_x _y _z) (Math|Vector|BreakVector _initial_location))
  (if (Variables|Default|GetIsOpen?)
    (Variables|Default|SetPower 2.0)
    (bind _newtrack_0 (Timeline|Timeline_0 Play)
      (:Update
        (Transformation|SetRelativeLocation (Variables|Default|GetDoor) (Math|Vector|MakeVector _x _y (Math|Float|Lerp _z (Variables|Default|GetDoorHeight) _newtrack_0)) false true)))
    (elif (> (Variables|Default|GetPower) 0.0)
      (Variables|Default|SetPower (- (Variables|Default|GetPower) DeltaSeconds))
      (else
        (Timeline|Timeline_0 Reverse)))))

(fn ConstructionScript)