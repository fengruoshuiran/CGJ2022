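; BP_Detection is a detection area that follows the player and reveals actors tagged "hide" while they overlap it.
; Each tick it teleports to the player character's location, or to BPdelayRef's DelayLocation when that object's LagMod is on.
; It gathers tagged actors at BeginPlay, unhiding them on overlap begin and hiding them on overlap end.
; The construction script scales the area's X and Y from InSphereRadius.
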(event OnComponentBeginOverlap(detectionarea)
  (params (OverlappedComponent :type Primitive%20Component%20Object%20Reference) (OtherActor :type Actor%20Object%20Reference) (OtherComp :type Primitive%20Component%20Object%20Reference) (OtherBodyIndex :type Integer) (bFromSweep :type Boolean) (SweepResult :type Hit%20Result%20Structure%20%28by%20ref%29))
  (if (Utilities|Array|ContainsItem (Variables|Default|GetActor%20With%20Tag%20List) OtherActor)
    (Rendering|SetActorHiddenInGame OtherActor false)))

(event OnComponentEndOverlap(detectionarea)
  (params (OverlappedComponent :type Primitive%20Component%20Object%20Reference) (OtherActor :type Actor%20Object%20Reference) (OtherComp :type Primitive%20Component%20Object%20Reference) (OtherBodyIndex :type Integer))
  (if (Utilities|Array|ContainsItem (Variables|Default|GetActor%20With%20Tag%20List) OtherActor)
    (Rendering|SetActorHiddenInGame OtherActor true)))

(event EventBeginPlay
  (bind _outactors (Actor|GetAllActorswithTag "hide"))
  (Variables|Default|SetActor%20With%20Tag%20List _outactors))

(event EventTick
  (params (DeltaSeconds :type Float%20%28single-precision%29))
  (bind _bpdelayref (Variables|Default|GetBPdelayRef))
  (if (Variables|/Game/BP/BP_DelaySystem.BP_DelaySystem_C|GetLagMod _bpdelayref)
    (Transformation|SetActorLocation (Variables|/Game/BP/BP_DelaySystem.BP_DelaySystem_C|GetDelayLocation _bpdelayref) false false)
    (else
      (Transformation|SetActorLocation (Transformation|GetActorLocation (Variables|Default|GetPlayerCharacterRef)) false false))))

(fn ConstructionScript
  (bind _in_sphere_radius (Variables|Default|GetIn%20Sphere%20Radius))
  (bind _returnvalue (/ _in_sphere_radius 7e+01))
  (Transformation|SetRelativeScale3D (Variables|Default|Getdetection%20area) (Math|Vector|MakeVector _returnvalue _returnvalue (Variables|Default|GetZ))))