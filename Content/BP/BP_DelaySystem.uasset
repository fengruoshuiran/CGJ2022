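; BP_DelaySystem simulates network lag as a gameplay mechanic by periodically snapping the player character back to an earlier position.
; A DoOnce-gated Tick loop picks wait and lag durations by level name, then records the character's location and spawns a BP_LagPoint marker at the player.
; When the lag window ends it teleports the character back, removes the marker and restarts, toggling LagMod on itself and its WB_Ping widget.
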(event Custom|TrackPlayerCharacter
  (Utilities|IsValid (Variables|Default|GetCharacterREF)))

(event Custom|DelayTeleport
  (Transformation|SetActorLocation (Variables|Default|GetCharacterREF) (Variables|Default|GetDelayLocation) false false))

(event EventBeginPlay
  (bind _returnvalue (UserInterface|CreateWidget "/Game/WB/WB_Ping.WB_Ping_C"))
  (UserInterface|Viewport|AddtoViewport _returnvalue 0)
  (Variables|Default|SetPing _returnvalue))

(event EventTick
  (params (DeltaSeconds :type Float%20%28single-precision%29))
  (bind _ping (Variables|Default|GetPing))
  (Utilities|FlowControl|DoOnce false :!label _label
    (:Completed
      (bind _returnvalue (Game|GetCurrentLevelName true))
      (Development|PrintString _returnvalue)
      (switch string _returnvalue
        (:Default
          (Variables|Default|SetDelay1 3.0 :!label _label_2)
          (Variables|Default|SetDelay2 2.0))
        (:LV_1
          (goto _label_2))
        (:LV_2
          (Variables|Default|SetDelay1 3.0)
          (Variables|Default|SetDelay2 2.0))
        (:LV_3
          (Variables|Default|SetDelay1 3.0)
          (Variables|Default|SetDelay2 3.0))
        (:LV_4
          (Variables|Default|SetDelay1 3.0)
          (Variables|Default|SetDelay2 3.0)))
      (Utilities|FlowControl|Delay (Variables|Default|GetDelay1))
      (Variables|Default|SetDelayLocation (Transformation|GetActorLocation (Variables|Default|GetCharacterREF)))
      (Variables|/Game/WB/WB_Ping.WB_Ping_C|SetLagMod _ping true)
      (Variables|Default|SetLagMod true)
      (bind _returnvalue_2 (Game|SpawnActorfromClass "/Game/BP/BP_LagPoint.BP_LagPoint_C" (Transformation|GetActorTransform (Game|Player|GetPlayerPawn 0)) "AlwaysSpawn" 0 0))
      (Variables|Default|SetLagPoint _returnvalue_2)
      (Utilities|FlowControl|Delay (Variables|Default|GetDelay2))
      (CallFunction|DelayTeleport)
      (Variables|/Game/WB/WB_Ping.WB_Ping_C|SetLagMod _ping false)
      (Variables|Default|SetLagMod false)
      (Actor|DestroyActor (Variables|Default|GetLagPoint))
      (goto _label Reset))))

(fn ConstructionScript)