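; BP_LevelInfo is a trigger actor that ends play as a win or a loss when the player reaches its box.
; On BeginPlay it caches the GM_main game mode.
; When the first player's pawn begins overlapping the Box, its Win flag selects whether the game mode's EventPlayerWin or EventPlayerLose is called.
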(event OnComponentBeginOverlap(Box)
  (params (OverlappedComponent :type Primitive%20Component%20Object%20Reference) (OtherActor :type Actor%20Object%20Reference) (OtherComp :type Primitive%20Component%20Object%20Reference) (OtherBodyIndex :type Integer) (bFromSweep :type Boolean) (SweepResult :type Hit%20Result%20Structure%20%28by%20ref%29))
  (bind _as_gm_main (Variables|Default|GetAs%20GM%20Main))
  (if (== OtherActor (Game|Player|GetPlayerPawn 0))
    (if (Variables|Default|Getwin)
      (Default|EventPlayerWin _as_gm_main)
      (else
        (Default|EventPlayerLose _as_gm_main)))))

(event EventBeginPlay
  (bind _asgm_main (Utilities|Casting|CastToGM_main (Game|GetGameMode)))
  (Variables|Default|SetAs%20GM%20Main _asgm_main))

(fn ConstructionScript)