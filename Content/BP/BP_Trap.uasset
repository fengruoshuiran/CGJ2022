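; BP_Trap is a trap actor whose Trap component moves vertically in a continuous loop from BeginPlay.
; BeginPlay slows the timeline's play rate, caches the component's world location and starts playback through a DoOnce.
; Each update offsets Z from that cached location by the scaled track value, and finishing restarts the timeline from the start.
; The graph contains no damage or overlap logic, and its delay and print nodes are unconnected.
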(event EventBeginPlay
  (Components|Timeline|SetPlayRate (Variables|Default|Get时间轴_0) 0.8)
  (Variables|Default|SetInitial%20location (Transformation|GetWorldLocation (Variables|Default|GetTrap)))
  (Utilities|FlowControl|DoOnce false
    (:Completed
      (Utilities|FlowControl|Sequence :!label _label
        (:then_0
          (bind _newtrack_0 (Timeline|时间轴_0 PlayFromStart)
            (:Update
              (Transformation|SetWorldLocation (Variables|Default|GetTrap) (Math|Vector|MakeVector (.X (Math|Vector|BreakVector (Variables|Default|GetInitial%20location))) (.Y (Math|Vector|BreakVector (Variables|Default|GetInitial%20location))) (+ (.Z (Math|Vector|BreakVector (Variables|Default|GetInitial%20location))) (* _newtrack_0 2e+01))) false false))
            (:Finished
              (goto _label))))))))

(fn ConstructionScript)