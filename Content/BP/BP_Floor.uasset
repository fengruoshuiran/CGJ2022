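; BP_Floor maintains a moving floor of BP_cube tiles around the player.
; On Tick it rounds the player's position, or BPDelaySystemRef's delayed location when LagMod is on, to a scaled grid cell.
; When the cell changes, it offsets a 7x7 template (ignoring the Radius input), spawning missing cubes and calling DisapperCube on out-of-range ones.
; Spawned cells are tracked in a list, while removal searches all BP_cube actors by grid location.
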(event Custom|Add%20single%20cube
  (params (SpawnLocation :type E%20Location%20Structure))
  (bind (_x _y) (Utilities|Struct|BreakELocation SpawnLocation))
  (bind _scale (Variables|Default|Getscale))
  (bind _scale_2 (Variables|Default|Getscale))
  (bind _elocation (Utilities|Struct|MakeELocation _x _y))
  (bind _returnvalue (/ _scale_2 1e+02))
  ;[1 1 1] add one sginle cube
  (Utilities|Array|Add (Variables|Default|GetSpawnedLocationList) _elocation)
  (bind _returnvalue_2 (Game|SpawnActorfromClass "/Game/BP/BaseAsset/BP_cube.BP_cube_C" (Math|Transform|MakeTransform (Math|Vector|MakeVector (* (Math|Conversions|ToFloat(Integer) _x) _scale) (* (Math|Conversions|ToFloat(Integer) _y) _scale) 0.0) "0, 0, 0" (Math|Vector|MakeVector _returnvalue _returnvalue _returnvalue)) "AdjustIfPossibleButDontSpawnIfColliding" 0 _elocation 0))
  (Utilities|Array|Add (Variables|Default|GetBP_cube_List) _returnvalue_2))

(event Custom|add%20%20cube%20area
  ;[1 1 1] add cube area
  (bind _player_area (CallFunction|LocationArea (Variables|Default|GetCurrentLocation) 1)) ; 计算需要生成地板的坐标
  (bind _output_get (Variables|Default|SetPlayer%20Area _player_area))
  (for _array_element _output_get ; 判断哪些地板已经生成
    (if (not (Utilities|Array|ContainsItem (Variables|Default|GetSpawnedLocationList) _array_element))
      (CallFunction|AddSingleCube _array_element)))
  (Utilities|Array|Clear (Variables|Default|Getlocation%20remove%20list))
  (for _array_element_2 (Variables|Default|GetSpawnedLocationList) ; 移除范围外的方块
    (Variables|Default|Setlocation%20temp _array_element_2)
    (if (not (Utilities|Array|ContainsItem (Variables|Default|GetPlayer%20Area) _array_element_2))
      (Utilities|Array|Add (Variables|Default|Getlocation%20remove%20list) (Variables|Default|Getlocation%20temp))
      (CallFunction|RemoveCube (Variables|Default|Getlocation%20temp))))
  (for _array_element_3 (Variables|Default|Getlocation%20remove%20list) ; 移除范围外的数据
    (Utilities|Array|RemoveItem (Variables|Default|GetSpawnedLocationList) _array_element_3)))

(event Custom|Remove%20cube
  (params (invalid%20location :type E%20Location%20Structure))
  ;[1 1 1] Remove cube
  (bind _outactors (Actor|GetAllActorsOfClass "/Game/BP/BaseAsset/BP_cube.BP_cube_C"))
  (for _array_element _outactors
    (if (Utilities|LocationEqual (Variables|/Game/BP/BaseAsset/BP_cube.BP_cube_C|Getlocation _array_element) invalid%20location)
      (Utilities|Array|RemoveItem (Variables|Default|GetBP_cube_List) _array_element)
      (Default|DisapperCube _array_element))))

(event EventTick
  (params (DeltaSeconds :type Float%20%28single-precision%29))
  (bind _playercharacterref (Variables|Default|GetPlayerCharacterRef))
  (bind _bp_delaysystem_ref (Variables|Default|GetBP_DelaySystem%20Ref))
  (bind _scale (Variables|Default|Getscale))
  (bind _returnvalue (Transformation|GetActorLocation _playercharacterref))
  (bind _lagmod (Variables|/Game/BP/BP_DelaySystem.BP_DelaySystem_C|GetLagMod _bp_delaysystem_ref))
  (bind _delaylocation (Variables|/Game/BP/BP_DelaySystem.BP_DelaySystem_C|GetDelayLocation _bp_delaysystem_ref))
  (bind _returnvalue_2 (select _lagmod _delaylocation _returnvalue))
  (bind (_x _y) (Math|Vector|BreakVector _returnvalue_2))
  (bind _returnvalue_3 (/ _y _scale))
  (bind _returnvalue_4 (/ _x _scale))
  (bind _returnvalue_5 (Math|Float|Round _returnvalue_3))
  (bind _returnvalue_6 (Math|Float|Round _returnvalue_4))
  (bind _elocation (Utilities|Struct|MakeELocation _returnvalue_6 _returnvalue_5))
  ;[1 0 0.06064] Tick
  (if (Utilities|IsValid (Variables|Default|GetPlayerCharacterREF))
    (if (not (Utilities|LocationEqual (Variables|Default|GetCurrentLocation) _elocation))
      (Variables|Default|SetCurrentLocation _elocation)
      (CallFunction|AddCubeArea))))

(event EventBeginPlay
  ;[0 1 0.1145] begine  play
  (Utilities|FlowControl|Sequence))

(fn ConstructionScript)

(fn LocationArea
  (params (player%20location :type E%20Location%20Structure) (radius :type Integer))
  (Utilities|Array|Clear (LocalVariables|GetPlayerArea))
  (for _array_element (LocalVariables|GetPlayerArea_Temp_7x7)
    (Utilities|Array|Add (LocalVariables|GetPlayerArea) (Utilities|LocationAdd _array_element player%20location)))
  (return (LocalVariables|GetPlayerArea)))